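; BP_FlyingCar is a flying car that travels in a loop along a spline path.
; On BeginPlay, the MoveActor timeline takes its play rate from CarSpeed; RandomizeSpeed randomizes that rate and adds a random start delay.
; The timeline's Animation track maps to spline distance, setting the Cube's world location and rotation with a fixed stretched scale.
; When finished, it restarts from the beginning after a zero-length delay.
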(event EventBeginPlay
  (bind _moveactor (Variables|Default|GetMoveActor))
  (bind _spline (Variables|FlyingCarProperties|GetSpline))
  (if (Variables|FlyingCarProperties|GetRandomizeSpeed)
    (bind _output_get (Variables|FlyingCarProperties|SetCarSpeed (Math|Random|RandomFloatinRange 1.0 5.0)))
    (Components|Timeline|SetPlayRate _moveactor _output_get)
    (Utilities|FlowControl|Delay (Math|Random|RandomFloatinRange 1.0 5.0))
    (bind _animation (Timeline|MoveActor PlayFromStart)
      (:Update
        (Transformation|SetWorldTransform (Variables|FlyingCarProperties|GetCube) (Math|Transform|MakeTransform (Spline|GetLocationatDistanceAlongSpline _spline (* (Spline|GetSplineLength _spline) _animation) "World") (Spline|GetRotationatDistanceAlongSpline _spline (* (Spline|GetSplineLength _spline) _animation) "World") "5.500000,2.500000,1.500000") false false))
      (:Finished
        (Utilities|FlowControl|Delay 0.0)
        (Timeline|MoveActor PlayFromStart)))
    (else
      (Components|Timeline|SetPlayRate _moveactor (Variables|FlyingCarProperties|GetCarSpeed))
      (Timeline|MoveActor PlayFromStart))))

(fn ConstructionScript)
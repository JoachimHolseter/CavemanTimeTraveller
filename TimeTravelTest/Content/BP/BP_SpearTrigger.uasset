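; Trigger volume that spawns a single spear when the Cavewoman runner character uses her special inside it.
; Box overlap opens and closes a gate on Tick, which matches the overlapping actor by display name and checks the player pawn's UsingSpecial flag.
; A DoOnce then spawns a scaled-down BP_Spear at the Arrow's transform.
; The construction script sets box scale and arrow placement from TriggerSize, SpearLocation and SpearRotation.
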(event OnComponentBeginOverlap(Box)
  (params (OverlappedComponent :type Primitive%20Component%20Object%20Reference) (OtherActor :type Actor%20Object%20Reference) (OtherComp :type Primitive%20Component%20Object%20Reference) (OtherBodyIndex :type Integer) (bFromSweep :type Boolean) (SweepResult :type Hit%20Result%20Structure%20%28by%20ref%29))
  (bind _arrow (Variables|Default|GetArrow))
  (bind _returnvalue (Transformation|GetWorldTransform _arrow))
  (Utilities|FlowControl|Gate true) ; enters at Open
)

(event OnComponentEndOverlap(Box)
  (params (OverlappedComponent :type Primitive%20Component%20Object%20Reference) (OtherActor :type Actor%20Object%20Reference) (OtherComp :type Primitive%20Component%20Object%20Reference) (OtherBodyIndex :type Integer))
  (bind _arrow (Variables|Default|GetArrow))
  (bind _returnvalue (Transformation|GetWorldTransform _arrow))
  (Utilities|FlowControl|Gate true) ; enters at Close
)

(event EventTick
  (params (DeltaSeconds :type Float%20%28single-precision%29))
  (bind _arrow (Variables|Default|GetArrow))
  (bind _returnvalue (Transformation|GetWorldTransform _arrow))
  (Utilities|FlowControl|Gate true
    (:Exit
      (if (Utilities|String|Contains (Utilities|GetDisplayName (stale OnComponentBeginOverlap(Box) OtherActor)) "Cavewoman")
        (bind _ascavewoman_character_runner (Utilities|Casting|CastToCavewomanCharacter_Runner (Game|Player|GetPlayerPawn 0)))
        (if (Variables|/Game/BP/CavewomanCharacter_Runner.CavewomanCharacter_Runner_C|GetUsingSpecial _ascavewoman_character_runner)
          (Utilities|FlowControl|DoOnce false
            (:Completed
              (Game|SpawnActorfromClass "/Game/BP/BP_Spear.BP_Spear_C" (Math|Transform|MakeTransform (.location _returnvalue) (.rotation _returnvalue) "0.600000,0.600000,0.600000") "Undefined" 0 0))))))))

(fn ConstructionScript
  (Transformation|SetRelativeScale3D (Variables|Default|GetBox) (Variables|Default|GetTriggerSize))
  (Transformation|SetRelativeTransform (Variables|Default|GetArrow) (Math|Transform|MakeTransform (Variables|Default|GetSpearLocation) (Variables|Default|GetSpearRotation) "2.000000,2.000000,2.000000") false false))
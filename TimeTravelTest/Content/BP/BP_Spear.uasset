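; BP_Spear is a runner-game spear that kills the player on hit or serves as a jump boost for the Cavewoman.
; Overlapping JumpBox while she is jumping launches her forward and up, with a DoOnce and delay limiting retriggers, and sets HasJumped.
; A spear hit before that sets the spear's IsDead, disabling the boost, and marks the Caveman or Cavewoman pawn dead, chosen by object name.
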(event OnComponentBeginOverlap(JumpBox)
  (params (OverlappedComponent :type Primitive%20Component%20Object%20Reference) (OtherActor :type Actor%20Object%20Reference) (OtherComp :type Primitive%20Component%20Object%20Reference) (OtherBodyIndex :type Integer) (bFromSweep :type Boolean) (SweepResult :type Hit%20Result%20Structure%20%28by%20ref%29))
  (if (not (Variables|Default|GetisDead))
    (bind _ascavewoman_character_runner (Utilities|Casting|CastToCavewomanCharacter_Runner (Game|Player|GetPlayerPawn 0)))
    (Utilities|IsValid _ascavewoman_character_runner
      (:Is%20Valid
        (if (Variables|/Game/BP/CavewomanCharacter_Runner.CavewomanCharacter_Runner_C|GetisJumping _ascavewoman_character_runner)
          (Utilities|FlowControl|DoOnce false :!label _label
            (:Completed
              (Variables|Default|SethasJumped true)
              (Character|LaunchCharacter _ascavewoman_character_runner "400.000000,0.000000,1000.000000" false false)
              (Utilities|FlowControl|Delay 1.0)
              (goto _label Reset))))))))

(event OnComponentHit(Spear)
  (params (HitComponent :type Primitive%20Component%20Object%20Reference) (OtherActor :type Actor%20Object%20Reference) (OtherComp :type Primitive%20Component%20Object%20Reference) (NormalImpulse :type Vector :default "0, 0, 0") (Hit :type Hit%20Result%20Structure%20%28by%20ref%29))
  (bind _returnvalue (Game|Player|GetPlayerPawn 0))
  (if (not (Variables|Default|GethasJumped))
    (Variables|Default|SetisDead true)
    (if (Utilities|String|Contains (Utilities|GetObjectName OtherActor) "Caveman")
      (bind _ascaveman_character_runner (Utilities|Casting|CastToCavemanCharacter_Runner _returnvalue))
      (Variables|/Game/BP/CavemanCharacter_Runner.CavemanCharacter_Runner_C|SetisDead _ascaveman_character_runner true)
      (elif (Utilities|String|Contains (Utilities|GetObjectName OtherActor) "Cavewoman")
        (bind _ascavewoman_character_runner (Utilities|Casting|CastToCavewomanCharacter_Runner _returnvalue))
        (Variables|/Game/BP/CavewomanCharacter_Runner.CavewomanCharacter_Runner_C|SetisDead _ascavewoman_character_runner true)))))

(fn ConstructionScript)
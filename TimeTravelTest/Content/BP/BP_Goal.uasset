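; BP_Goal is the level's finish trigger, ending the run when the Caveman overlaps its Box.
; The overlapping actor is identified by a display-name substring check, and a DoOnce keeps the finish from repeating.
; It marks itself activated, stops the timer and sets HasFinished on the CavemanPlayerController, then calls CalculateScore on the first top-level PlayerWidget it finds.
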(event OnComponentBeginOverlap(Box)
  (params (OverlappedComponent :type Primitive%20Component%20Object%20Reference) (OtherActor :type Actor%20Object%20Reference) (OtherComp :type Primitive%20Component%20Object%20Reference) (OtherBodyIndex :type Integer) (bFromSweep :type Boolean) (SweepResult :type Hit%20Result%20Structure%20%28by%20ref%29))
  (if (Utilities|String|Contains (Utilities|GetDisplayName OtherActor) "Caveman")
    (Utilities|FlowControl|DoOnce false
      (:Completed
        (Variables|Default|SetisActivated true)
        (bind _ascaveman_player_controller (Utilities|Casting|CastToCavemanPlayerController (Game|GetPlayerController 0)))
        (Default|StopTimer _ascaveman_player_controller)
        (Variables|/Game/BP/CavemanCharacter/CavemanPlayerController.CavemanPlayerController_C|SethasFinished _ascaveman_player_controller true)
        (bind _foundwidgets (Widget|GetAllWidgetsOfClass "/Game/UMG/PlayerWidget.PlayerWidget_C" true))
        (Default|CalculateScore (Utilities|Array|Get(acopy) _foundwidgets))))))

(fn ConstructionScript)
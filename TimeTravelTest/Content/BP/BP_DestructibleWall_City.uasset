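; BP_DestructibleWall_City is a stone wall that shatters when the Caveman player uses their special (dash) while inside its trigger.
; TriggerBox overlaps set a presence flag by matching "Caveman" in the actor name, and Tick polls it, casting to BP_Caveman_Platformer to check UsingSpecial.
; The one-shot break disables BlockVolume collision, enables physics on the destructible mesh, applies radial damage and a delayed force, then destroys the actor.
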(event OnComponentEndOverlap(TriggerBox)
  (params (OverlappedComponent :type Primitive%20Component%20Object%20Reference) (OtherActor :type Actor%20Object%20Reference) (OtherComp :type Primitive%20Component%20Object%20Reference) (OtherBodyIndex :type Integer))
  ;[1 1 1] End overlap
  (if (Utilities|String|Contains (Utilities|GetObjectName OtherActor) "Caveman")
    (Variables|Default|SetPlayerInTrigger false)))

(event OnComponentBeginOverlap(TriggerBox)
  (params (OverlappedComponent :type Primitive%20Component%20Object%20Reference) (OtherActor :type Actor%20Object%20Reference) (OtherComp :type Primitive%20Component%20Object%20Reference) (OtherBodyIndex :type Integer) (bFromSweep :type Boolean) (SweepResult :type Hit%20Result%20Structure%20%28by%20ref%29))
  ;[1 1 1] On Component Begin Overlap (TriggerBox)
  (if (Utilities|String|Contains (Utilities|GetObjectName OtherActor) "Caveman")
    (Variables|Default|SetPlayerInTrigger true)))

(event EventTick
  (params (DeltaSeconds :type Float%20%28single-precision%29))
  ;[1 1 1] Break if player is dashing
  (if (Variables|Default|GetPlayerInTrigger)
    (bind _asbp_caveman_platformer (Utilities|Casting|CastToBP_Caveman_Platformer (stale OnComponentBeginOverlap(TriggerBox) OtherActor)))
    (if (Variables|/Game/BP/CavemanCharacter/BP_Caveman_Platformer.BP_Caveman_Platformer_C|GetUsingSpecial _asbp_caveman_platformer)
      (Variables|Default|SetBoxBroken true)
      (Utilities|FlowControl|DoOnce false
        (:Completed
          (Collision|SetCollisionProfileName (Variables|Default|GetBlockVolume) "NoCollision" :!class /Script/Engine.PrimitiveComponent)
          (Physics|SetSimulatePhysics (Variables|Default|GetStone_Destructable_Mesh_DM) true)
          (Class|DestructibleComponent|ApplyRadiusDamage (Variables|Default|GetStone_Destructable_Mesh_DM) 1e+03 (Transformation|GetActorLocation) 0.0 5e+04 true)
          (Utilities|FlowControl|Delay 0.2)
          (Physics|AddForce (Variables|Default|GetStone_Destructable_Mesh_DM) "5000.000000,5000.000000,5000.000000" "None" false)
          (Utilities|FlowControl|Delay 2.0)
          (Actor|DestroyActor))))))

(fn ConstructionScript)
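; BP_Drone1 is a city drone actor that hovers in place with spinning rotor blades.
; On BeginPlay it stores its start location, waits a random short delay to desync instances, then plays the Float timeline to offset its height.
; Tick yaws four blade components by a fixed, frame-rate-dependent step.
; It also caches the first BP_Caveman_Platformer as PlayerRef, which this graph never uses.
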(event EventBeginPlay
  (Variables|Default|SetStartPos (Transformation|GetWorldLocation (Variables|Default|GetDefaultSceneRoot)))
  (bind _outactors (Actor|GetAllActorsOfClass "/Game/BP/CavemanCharacter/BP_Caveman_Platformer.BP_Caveman_Platformer_C"))
  (Variables|Default|SetPlayerRef (Utilities|Array|Get(acopy) _outactors))
  (Utilities|FlowControl|Delay (Math|Random|RandomFloatinRange 0.0 2.0))
  (bind _posistion (Timeline|Float PlayFromStart)
    (:Update
      (Transformation|SetActorLocation (Math|Vector|MakeVector (.x (Variables|Default|GetStartPos)) (.y (Variables|Default|GetStartPos)) (+ (.z (Variables|Default|GetStartPos)) _posistion)) false false))))

(event EventTick
  (params (DeltaSeconds :type Float%20%28single-precision%29))
  (Transformation|AddLocalRotation (Variables|Default|GetBlade1) "0.000000,45.000000,0.000000" false false))

(fn ConstructionScript)
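; City door actor that the caveman player opens and closes with a button, optionally closing itself at BeginPlay.
; Tick polls the player's Interacting flag inside the trigger box, and a DoOnce feeds a FlipFlop that alternates two timelines sliding the door along Z.
; Button and lights turn red with the prompt hidden during movement, then a delayed reset turns them green, shows the prompt and re-arms the DoOnce.
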(event OnComponentBeginOverlap(TriggerBox)
  (params (OverlappedComponent :type Primitive%20Component%20Object%20Reference) (OtherActor :type Actor%20Object%20Reference) (OtherComp :type Primitive%20Component%20Object%20Reference) (OtherBodyIndex :type Integer) (bFromSweep :type Boolean) (SweepResult :type Hit%20Result%20Structure%20%28by%20ref%29))
  ;[1 1 1] If player is in range of trigger, show interact text
  (Variables|Default|SetPlayerInTrigger true)
  (Rendering|SetVisibility (Variables|Default|GetTextRender1) true false))

(event OnComponentEndOverlap(TriggerBox)
  (params (OverlappedComponent :type Primitive%20Component%20Object%20Reference) (OtherActor :type Actor%20Object%20Reference) (OtherComp :type Primitive%20Component%20Object%20Reference) (OtherBodyIndex :type Integer))
  ;[1 1 1] If player is in range of trigger, show interact text
  (Variables|Default|SetPlayerInTrigger false)
  (Rendering|SetVisibility (Variables|Default|GetTextRender1) false false))

(event Custom|ResetDoOnce
  (bind _door (Variables|Default|GetDoor))
  (bind _door_2 (Variables|Default|GetDoor))
  (bind _relativelocation (Variables|/Script/Engine.SceneComponent|GetRelativeLocation _door))
  (bind _relativelocation_2 (Variables|/Script/Engine.SceneComponent|GetRelativeLocation _door_2))
  ;[1 1 1] Reset DoOnce and set colors and interact text to visible
  (Utilities|FlowControl|Delay 1.0)
  (Rendering|Material|SetMaterial (Variables|Default|GetButton) 0 "/Game/MT/GreenButtonMTL.GreenButtonMTL")
  (Rendering|Components|Light|SetLightColor (Variables|Default|GetPointLight) "(R=0.000000,G=1.000000,B=0.000000,A=1.000000)" true)
  (Rendering|SetVisibility (Variables|Default|GetTextRender1) true false)
  ;[1 1 1] If player is interacting inside the trigger
  (Utilities|FlowControl|DoOnce false) ; enters at Reset
)

(event Custom|CloseDoor
  (bind _door (Variables|Default|GetDoor))
  (bind _relativelocation (Variables|/Script/Engine.SceneComponent|GetRelativeLocation _door))
  ;[1 1 1] move the door with the timeline
  (bind _doorpos (Timeline|MoveDoor PlayFromStart)
    (:Update
      (Transformation|SetRelativeLocation _door (Math|Vector|MakeVector (.x _relativelocation) (.y _relativelocation) _doorpos) false false)
      ;[1 1 1] Set colors and toggle interact text
      (Rendering|Material|SetMaterial (Variables|Default|GetButton) 0 "/Game/MT/RedButtonMTL.RedButtonMTL")
      (Rendering|Components|Light|SetLightColor (Variables|Default|GetPointLight) "(R=1.000000,G=0.000000,B=0.000000,A=1.000000)" true)
      (Rendering|SetVisibility (Variables|Default|GetTextRender1) false false))
    (:Finished
      (Variables|Default|SetDoorClosed true)
      (CallFunction|ResetDoOnce))))

(event Custom|OpenDoor
  (bind _door (Variables|Default|GetDoor))
  (bind _relativelocation (Variables|/Script/Engine.SceneComponent|GetRelativeLocation _door))
  ;[1 1 1] move the door with the timeline
  (bind _doorpos (Timeline|Timeline_0 ReverseFromEnd)
    (:Update
      (Transformation|SetRelativeLocation _door (Math|Vector|MakeVector (.x _relativelocation) (.y _relativelocation) _doorpos) false false)
      ;[1 1 1] Set colors and toggle interact text
      (Rendering|Material|SetMaterial (Variables|Default|GetButton) 0 "/Game/MT/RedButtonMTL.RedButtonMTL")
      (Rendering|Components|Light|SetLightColor (Variables|Default|GetPointLight) "(R=1.000000,G=0.000000,B=0.000000,A=1.000000)" true)
      (Rendering|SetVisibility (Variables|Default|GetTextRender1) false false))
    (:Finished
      (Variables|Default|SetDoorClosed false)
      (CallFunction|ResetDoOnce))))

(event EventTick
  (params (DeltaSeconds :type Float%20%28single-precision%29))
  (bind _door (Variables|Default|GetDoor))
  (bind _door_2 (Variables|Default|GetDoor))
  (bind _relativelocation (Variables|/Script/Engine.SceneComponent|GetRelativeLocation _door))
  (bind _relativelocation_2 (Variables|/Script/Engine.SceneComponent|GetRelativeLocation _door_2))
  ;[1 1 1] If player is interacting inside the trigger
  (if (Variables|Default|GetPlayerInTrigger)
    (bind _asbp_caveman_platformer (Utilities|Casting|CastToBP_Caveman_Platformer (Game|GetPlayerCharacter 0)))
    (if (Variables|/Game/BP/CavemanCharacter/BP_Caveman_Platformer.BP_Caveman_Platformer_C|Getinteracting _asbp_caveman_platformer)
      (Utilities|FlowControl|DoOnce false
        (:Completed
          (Utilities|FlowControl|FlipFlop
            (:A
              ;[1 1 1] move the door with the timeline
              (bind _doorpos (Timeline|Timeline_0 PlayFromStart)
                (:Update
                  (Transformation|SetRelativeLocation _door (Math|Vector|MakeVector (.x _relativelocation) (.y _relativelocation) _doorpos) false false)
                  ;[1 1 1] Set colors and toggle interact text
                  (Rendering|Material|SetMaterial (Variables|Default|GetButton) 0 "/Game/MT/RedButtonMTL.RedButtonMTL")
                  (Rendering|Components|Light|SetLightColor (Variables|Default|GetPointLight) "(R=1.000000,G=0.000000,B=0.000000,A=1.000000)" true)
                  (Rendering|SetVisibility (Variables|Default|GetTextRender1) false false))
                (:Finished
                  (Variables|Default|SetDoorClosed false)
                  (CallFunction|ResetDoOnce))))
            (:B
              (bind _doorpos_2 (Timeline|MoveDoor PlayFromStart)
                (:Update
                  (Transformation|SetRelativeLocation _door_2 (Math|Vector|MakeVector (.x _relativelocation_2) (.y _relativelocation_2) _doorpos_2) false false)
                  (Rendering|Material|SetMaterial (Variables|Default|GetButton) 0 "/Game/MT/RedButtonMTL.RedButtonMTL")
                  (Rendering|Components|Light|SetLightColor (Variables|Default|GetPointLight) "(R=1.000000,G=0.000000,B=0.000000,A=1.000000)" true)
                  (Rendering|SetVisibility (Variables|Default|GetTextRender1) false false))
                (:Finished
                  (Variables|Default|SetDoorClosed true)
                  (CallFunction|ResetDoOnce))))))))))

(event EventBeginPlay
  (if (Variables|Default|GetStartClosed)
    (CallFunction|CloseDoor)))

(fn ConstructionScript)
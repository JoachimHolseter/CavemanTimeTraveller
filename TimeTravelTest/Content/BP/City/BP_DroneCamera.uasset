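; BP_DroneCamera is a city drone with a camera that hovers and watches the platformer caveman.
; After a random start delay, a timeline offsets its height from the spawn position.
; Tick spins the blades, film reels and spinner, and yaws the camera toward the player's mesh using a look-at rotation.
; A delayed FlipFlop on Tick alternates three spotlights between blue and red like a siren.
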(event EventBeginPlay
  (Variables|Default|SetStartPos (Transformation|GetWorldLocation (Variables|Default|GetDefaultSceneRoot)))
  (bind _outactors (Actor|GetAllActorsOfClass "/Game/BP/CavemanCharacter/BP_Caveman_Platformer.BP_Caveman_Platformer_C"))
  (Variables|Default|SetPlayerRef (Utilities|Array|Get(acopy) _outactors))
  (Utilities|FlowControl|Delay (Math|Random|RandomFloatinRange 0.0 2.0))
  (bind _posistion (Timeline|Float PlayFromStart)
    (:Update
      (Transformation|SetActorLocation (Math|Vector|MakeVector (.x (Variables|Default|GetStartPos)) (.y (Variables|Default|GetStartPos)) (+ (.z (Variables|Default|GetStartPos)) _posistion)) false false))))

(event EventTick
  (params (DeltaSeconds :type Float%20%28single-precision%29))
  (bind _returnvalue (Transformation|GetActorLocation))
  (bind _playerref (Variables|Default|GetPlayerRef))
  (bind _spotlight (Variables|Default|GetSpotLight))
  (bind _mesh (Variables|/Script/Engine.Character|GetMesh _playerref))
  (bind _returnvalue_2 (Transformation|GetWorldLocation _mesh))
  (bind _returnvalue_3 (Math|Rotator|FindLookatRotation _returnvalue _returnvalue_2))
  (Utilities|FlowControl|Sequence
    (:then_0
      (Transformation|AddLocalRotation (Variables|Default|GetFilm) "0, 0,1.000000" false false)
      (Transformation|AddLocalRotation (Variables|Default|GetSpinner) "0, 0,3.000000" false false)
      (Transformation|SetRelativeRotation (Variables|Default|GetCamera) (Math|Rotator|MakeRotator (.roll _returnvalue_3) 0.0 (- (.yaw _returnvalue_3) 9e+01)) false false)
      (Transformation|AddLocalRotation (Variables|Default|GetBlade1) "0.000000,45.000000,0.000000" false false))
    (:then_1
      (Utilities|FlowControl|Delay 0.2)
      (Utilities|FlowControl|FlipFlop
        (:A
          (Rendering|Components|Light|SetLightColor _spotlight "(R=0.000000,G=0.020532,B=1.000000,A=1.000000)" true))
        (:B
          (Rendering|Components|Light|SetLightColor _spotlight "(R=1.000000,G=0.000000,B=0.000000,A=1.000000)" true))))))

(fn ConstructionScript)
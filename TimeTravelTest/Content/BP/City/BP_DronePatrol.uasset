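; Patrol drone actor that flies its body back and forth between its start position and a patrol point while its four blades spin.
; After an initial delay, MoveActor eases the Body to PatrolPoint and back over Time, then calls itself to loop endlessly.
; Tick rotates the four blade components by a fixed yaw step each frame, so spin speed depends on frame rate.
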(event Custom|MoveActor
  (Components|MoveComponentTo (Variables|Default|GetBody) (Variables|Default|GetPatrolPoint) "0, 0, 0" true true (Variables|Default|GetTime) false)
  (Components|MoveComponentTo (Variables|Default|GetBody) (Variables|Default|GetStartLocation) "0, 0, 0" true true (Variables|Default|GetTime) false)
  (CallFunction|MoveActor))

(event EventBeginPlay
  (Variables|Default|SetStartLocation (Variables|/Script/Engine.SceneComponent|GetRelativeLocation (Variables|Default|GetBody)))
  (Utilities|FlowControl|Delay (Variables|Default|GetDelay))
  (CallFunction|MoveActor))

(event EventTick
  (params (DeltaSeconds :type Float%20%28single-precision%29))
  (Transformation|AddLocalRotation (Variables|Default|GetBlade1) "0.000000,45.000000,0.000000" false false))

(fn ConstructionScript)
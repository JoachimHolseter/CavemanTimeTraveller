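; BP_PoliceCarStationary is a city police car that hovers in place while turning to face the player.
; On BeginPlay it stores its start location, caches the first BP_Caveman_Platformer as the player, and plays a Float timeline that offsets its height from that start point.
; Each tick it rotates toward the player with a look-at rotation, halving the pitch so it tilts less steeply.
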(event EventBeginPlay
  (Variables|Default|SetStartPos (Transformation|GetWorldLocation (Variables|FlyingCarProperties|GetDefaultSceneRoot)))
  (bind _outactors (Actor|GetAllActorsOfClass "/Game/BP/CavemanCharacter/BP_Caveman_Platformer.BP_Caveman_Platformer_C"))
  (Variables|Default|SetPlayerReference (Utilities|Array|Get(acopy) _outactors))
  (bind _posistion (Timeline|Float Play)
    (:Update
      (Transformation|SetActorLocation (Math|Vector|MakeVector (.x (Variables|Default|GetStartPos)) (.y (Variables|Default|GetStartPos)) (+ (.z (Variables|Default|GetStartPos)) _posistion)) false false))))

(event EventTick
  (params (DeltaSeconds :type Float%20%28single-precision%29))
  (bind _returnvalue (Transformation|GetActorLocation))
  (bind _playerreference (Variables|Default|GetPlayerReference))
  (bind _returnvalue_2 (Transformation|GetActorLocation _playerreference))
  (bind _returnvalue_3 (Math|Rotator|FindLookatRotation _returnvalue _returnvalue_2))
  (Transformation|SetActorRotation (Math|Rotator|MakeRotator (.roll _returnvalue_3) (/ (.pitch _returnvalue_3) 2.0) (.yaw _returnvalue_3))))

(fn ConstructionScript)
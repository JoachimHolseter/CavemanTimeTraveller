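; BP_MultipleFlyingCar is a city actor that moves flying car meshes along a spline in an endless loop.
; On BeginPlay it sets the timeline play rate from CarSpeed, optionally randomizing that speed and adding a random start delay.
; The MoveActor timeline maps its value to spline distance and gives all three meshes one shared transform, taking roll and pitch from the spline, yaw from ForwardRotation and scale from Size.
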(event EventBeginPlay
  (bind _moveactor (Variables|Default|GetMoveActor))
  (bind _spline (Variables|FlyingCarProperties|GetSpline))
  (if (Variables|FlyingCarProperties|GetRandomizeSpeed)
    (bind _output_get (Variables|FlyingCarProperties|SetCarSpeed (Math|Random|RandomFloatinRange 1.0 5.0)))
    (Components|Timeline|SetPlayRate _moveactor _output_get)
    (Utilities|FlowControl|Delay (Math|Random|RandomFloatinRange 1.0 5.0))
    (bind _animation (Timeline|MoveActor PlayFromStart)
      (:Update
        (Transformation|SetWorldTransform (Variables|Default|GetStaticMesh) (Math|Transform|MakeTransform (Spline|GetLocationatDistanceAlongSpline _spline (* (Spline|GetSplineLength _spline) _animation) "World") (Math|Rotator|MakeRotator (.roll (Spline|GetRotationatDistanceAlongSpline _spline (* (Spline|GetSplineLength _spline) _animation) "World")) (.pitch (Spline|GetRotationatDistanceAlongSpline _spline (* (Spline|GetSplineLength _spline) _animation) "World")) (Variables|FlyingCarProperties|GetForwardRotation)) (Variables|FlyingCarProperties|GetSize)) false false))
      (:Finished
        (Utilities|FlowControl|Delay 0.0)
        (Timeline|MoveActor PlayFromStart)))
    (else
      (Components|Timeline|SetPlayRate _moveactor (Variables|FlyingCarProperties|GetCarSpeed))
      (Timeline|MoveActor PlayFromStart))))

(fn ConstructionScript)
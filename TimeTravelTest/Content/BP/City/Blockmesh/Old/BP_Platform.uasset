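; City platform actor for the runner characters that kills the player when its collision component is hit.
; The hit event identifies the other actor by a "Caveman" or "Cavewoman" substring in its object name.
; It then casts player pawn 0, rather than the hit actor, to the matching runner character class and sets its IsDead flag.
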(event OnComponentHit(Collision)
  (params (HitComponent :type Primitive%20Component%20Object%20Reference) (OtherActor :type Actor%20Object%20Reference) (OtherComp :type Primitive%20Component%20Object%20Reference) (NormalImpulse :type Vector :default "0, 0, 0") (Hit :type Hit%20Result%20Structure%20%28by%20ref%29))
  (bind _returnvalue (Game|Player|GetPlayerPawn 0))
  (if (Utilities|String|Contains (Utilities|GetObjectName OtherActor) "Caveman")
    (bind _ascaveman_character_runner (Utilities|Casting|CastToCavemanCharacter_Runner _returnvalue))
    (Variables|/Game/BP/CavemanCharacter/CavemanCharacter_Runner.CavemanCharacter_Runner_C|SetisDead _ascaveman_character_runner true)
    (elif (Utilities|String|Contains (Utilities|GetObjectName OtherActor) "Cavewoman")
      (bind _ascavewoman_character_runner (Utilities|Casting|CastToCavewomanCharacter_Runner _returnvalue))
      (Variables|/Game/BP/CavemanCharacter/CavewomanCharacter_Runner.CavewomanCharacter_Runner_C|SetisDead _ascavewoman_character_runner true))))

(fn ConstructionScript)
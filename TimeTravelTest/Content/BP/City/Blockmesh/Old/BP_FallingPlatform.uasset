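; Falling platform actor whose static mesh drops under physics after something overlaps its trigger box, then returns to its starting transform.
; Overlap events set a flag that Tick polls to start a delay before breaking, which leaving the box does not cancel.
; Breaking enables physics simulation, guarded by a bool and a DoOnce.
; After a reset delay, physics turns off, the transform saved at BeginPlay is restored and both guards re-arm.
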(event OnComponentEndOverlap(TriggerBox)
  (params (OverlappedComponent :type Primitive%20Component%20Object%20Reference) (OtherActor :type Actor%20Object%20Reference) (OtherComp :type Primitive%20Component%20Object%20Reference) (OtherBodyIndex :type Integer))
  (Variables|Default|SetinTrigger false))

(event OnComponentBeginOverlap(TriggerBox)
  (params (OverlappedComponent :type Primitive%20Component%20Object%20Reference) (OtherActor :type Actor%20Object%20Reference) (OtherComp :type Primitive%20Component%20Object%20Reference) (OtherBodyIndex :type Integer) (bFromSweep :type Boolean) (SweepResult :type Hit%20Result%20Structure%20%28by%20ref%29))
  (Variables|Default|SetinTrigger true))

(event Custom|Break
  (if (not (Variables|Default|GetBoxBroken))
    (Variables|Default|SetBoxBroken true)
    (Utilities|FlowControl|DoOnce false
      (:Completed
        (Physics|SetSimulatePhysics (Variables|Default|GetStaticMesh) true)
        (Utilities|FlowControl|Delay (Variables|Default|GetResetTime))
        (CallFunction|Reset)
        (Physics|SetSimulatePhysics (Variables|Default|GetStaticMesh) false)))))

(event Custom|Reset
  (Physics|SetSimulatePhysics (Variables|Default|GetStaticMesh) false)
  (Transformation|SetWorldTransform (Variables|Default|GetStaticMesh) (Variables|Default|GetStartPos) false false)
  (Variables|Default|SetBoxBroken false)
  (CallFunction|ResetDoOnce))

(event Custom|ResetDoOnce
  (Utilities|FlowControl|DoOnce false) ; enters at Reset
)

(event EventTick
  (params (DeltaSeconds :type Float%20%28single-precision%29))
  (if (Variables|Default|GetinTrigger)
    (Utilities|FlowControl|Delay (Variables|Default|GetTime))
    (CallFunction|Break)))

(event EventBeginPlay
  (Variables|Default|SetStartPos (Transformation|GetWorldTransform (Variables|Default|GetStaticMesh))))

(fn ConstructionScript)
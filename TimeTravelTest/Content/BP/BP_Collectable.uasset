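; Collectable pickup that records itself as found in PuzzleGamemode's Level 1 flags, then destroys itself.
; The construction script applies a configurable mesh and material array to each instance.
; After a random start delay, a timeline offsets its height from the start position.
; On sphere overlap with an actor whose name contains "Caveman", CollectableNumber selects which of three flags to set and prints a message.
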(event OnComponentBeginOverlap(Sphere)
  (params (OverlappedComponent :type Primitive%20Component%20Object%20Reference) (OtherActor :type Actor%20Object%20Reference) (OtherComp :type Primitive%20Component%20Object%20Reference) (OtherBodyIndex :type Integer) (bFromSweep :type Boolean) (SweepResult :type Hit%20Result%20Structure%20%28by%20ref%29))
  (bind _collectablenumber (Variables|Default|GetCollectableNumber))
  (if (Utilities|String|Contains (Utilities|GetObjectName OtherActor) "Caveman")
    (bind _aspuzzle_gamemode (Utilities|Casting|CastToPuzzleGamemode (Game|GetGameMode)))
    (if (== _collectablenumber 1)
      (Variables|/Game/BP/Logic/PuzzleGamemode.PuzzleGamemode_C|SetCollectable1Level1 _aspuzzle_gamemode true)
      (Development|PrintString "Collectable 1 Found")
      (Actor|DestroyActor :!label _label)
      (elif (== _collectablenumber 2)
        (Variables|/Game/BP/Logic/PuzzleGamemode.PuzzleGamemode_C|SetCollectable2Level1 _aspuzzle_gamemode true)
        (Development|PrintString "Collectable 2 Found")
        (goto _label)
        (elif (== _collectablenumber 3)
          (Variables|/Game/BP/Logic/PuzzleGamemode.PuzzleGamemode_C|SetCollectable3Level1 _aspuzzle_gamemode true)
          (Development|PrintString "Collectable 3 Found")
          (goto _label))))))

(event EventBeginPlay
  (Variables|Default|SetStartPos (Transformation|GetWorldLocation (Variables|Default|GetDefaultSceneRoot)))
  (Utilities|FlowControl|Delay (Math|Random|RandomFloatinRange 0.0 2.0))
  (bind _posistion (Timeline|Timeline_0 PlayFromStart)
    (:Update
      (Transformation|SetActorLocation (Math|Vector|MakeVector (.x (Variables|Default|GetStartPos)) (.y (Variables|Default|GetStartPos)) (+ (.z (Variables|Default|GetStartPos)) _posistion)) false false))))

(fn ConstructionScript
  (bind _staticmesh (Variables|Default|GetStaticMesh))
  (Components|StaticMesh|SetStaticMesh _staticmesh (Variables|Default|GetMesh))
  (for (_array_element _array_index) (Variables|Default|GetMesh%20Materials)
    (Rendering|Material|SetMaterial _staticmesh _array_index _array_element)))
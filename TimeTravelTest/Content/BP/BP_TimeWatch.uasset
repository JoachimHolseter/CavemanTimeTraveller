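; Time watch pickup that unlocks the time travel device for the platformer caveman player.
; A timeline started on BeginPlay offsets its height from the start position, while Tick spins three meshes at different yaw rates, not scaled by delta time.
; On the first sphere overlap by BP_Caveman_Platformer, it calls TimeTravelDeviceUnlocked and clears its four meshes rather than destroying the actor.
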(event OnComponentBeginOverlap(Sphere)
  (params (OverlappedComponent :type Primitive%20Component%20Object%20Reference) (OtherActor :type Actor%20Object%20Reference) (OtherComp :type Primitive%20Component%20Object%20Reference) (OtherBodyIndex :type Integer) (bFromSweep :type Boolean) (SweepResult :type Hit%20Result%20Structure%20%28by%20ref%29))
  (bind _asbp_caveman_platformer (Utilities|Casting|CastToBP_Caveman_Platformer OtherActor))
  (Utilities|FlowControl|DoOnce false
    (:Completed
      (Default|TimeTravelDeviceUnlocked _asbp_caveman_platformer)
      (Components|StaticMesh|SetStaticMesh (Variables|Default|GetStaticMesh2) 0)
      (Components|StaticMesh|SetStaticMesh (Variables|Default|GetStaticMesh) 0)
      (Components|StaticMesh|SetStaticMesh (Variables|Default|GetStaticMesh3) 0)
      (Components|StaticMesh|SetStaticMesh (Variables|Default|GetStaticMesh1) 0))))

(event EventBeginPlay
  (Variables|Default|SetStartPos (Transformation|GetWorldLocation (Variables|Default|GetDefaultSceneRoot)))
  (bind _posistion (Timeline|Timeline_0 PlayFromStart)
    (:Update
      (Transformation|SetActorLocation (Math|Vector|MakeVector (.x (Variables|Default|GetStartPos)) (.y (Variables|Default|GetStartPos)) (+ (.z (Variables|Default|GetStartPos)) _posistion)) false false))))

(event Collision|EventActorBeginOverlap
  (params (OtherActor :type Actor%20Object%20Reference)))

(event EventTick
  (params (DeltaSeconds :type Float%20%28single-precision%29))
  (Transformation|AddLocalRotation (Variables|Default|GetStaticMesh3) "1.000000,0.000000,0.000000" false false)
  (Transformation|AddLocalRotation (Variables|Default|GetStaticMesh2) "1.200000,0.000000,0.000000" false false)
  (Transformation|AddLocalRotation (Variables|Default|GetStaticMesh1) "-2.000000,0.000000,0.000000" false false))

(fn ConstructionScript)
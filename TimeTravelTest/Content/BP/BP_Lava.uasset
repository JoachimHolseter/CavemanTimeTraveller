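; Lava hazard actor that kills the caveman player character on contact with its trigger box.
; On overlap it matches "Caveman" in the actor's name, then uses the level name to cast to the runner ("RunnerTest") or puzzle character and set IsDead.
; The construction script applies the configurable scale and lava material to the plane and derives the box extent from that scale and TriggerBoxZ.
; Hit and activation events only print debug text.
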(event OnComponentBeginOverlap(Box)
  (params (OverlappedComponent :type Primitive%20Component%20Object%20Reference) (OtherActor :type Actor%20Object%20Reference) (OtherComp :type Primitive%20Component%20Object%20Reference) (OtherBodyIndex :type Integer) (bFromSweep :type Boolean) (SweepResult :type Hit%20Result%20Structure%20%28by%20ref%29))
  (if (Utilities|String|Contains (Utilities|GetObjectName OtherActor) "Caveman")
    (bind _returnvalue (Game|GetCurrentLevelName true))
    (if (Utilities|Enum|Equal(Enum) _returnvalue "RunnerTest")
      (bind _ascaveman_character_runner (Utilities|Casting|CastToCavemanCharacter_Runner OtherActor))
      (Variables|/Game/BP/CavemanCharacter_Runner.CavemanCharacter_Runner_C|SetisDead _ascaveman_character_runner true)
      (else
        (bind _ascaveman_character_puzzle (Utilities|Casting|CastToCavemanCharacter_Puzzle OtherActor))
        (Variables|/Game/BP/CavemanCharacter_Puzzle.CavemanCharacter_Puzzle_C|SetisDead _ascaveman_character_puzzle true)))))

(event OnComponentHit(Box)
  (params (HitComponent :type Primitive%20Component%20Object%20Reference) (OtherActor :type Actor%20Object%20Reference) (OtherComp :type Primitive%20Component%20Object%20Reference) (NormalImpulse :type Vector :default "0, 0, 0") (Hit :type Hit%20Result%20Structure%20%28by%20ref%29))
  (Development|PrintString "Hello"))

(event OnComponentActivated(Box)
  (params (Component :type Actor%20Component%20Object%20Reference) (bReset :type Boolean))
  (Development|PrintString "Hello"))

(fn ConstructionScript
  (bind _planescale (Variables|Default|GetPlaneScale))
  (Transformation|SetWorldScale3D (Variables|Default|GetPlane) (Math|Vector|MakeVector (.x _planescale) (.y _planescale) (.z _planescale)))
  (Rendering|Material|SetMaterial (Variables|Default|GetPlane) 0 (Variables|Default|GetLavaMaterial))
  (Components|Box|SetBoxExtent (Variables|Default|GetBox) (Math|Vector|MakeVector (.x _planescale) (.y _planescale) (/ (Variables|Default|GetTriggerBoxZ) 1e+02)) true))
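; Save game Blueprint that stores the player name, intro level collectables, level scores and ratings, and per-level high score tables.
; Its only event, PrintValues, is a debug dump that prints these values and today's date on screen in color.
; Nested loops print the level 0 entries' times and names, with the level 1 count printed inside the loop.
; IntToText contains an unconnected expression that zero-pads three integers into a 00:00.00 time string.
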(event Custom|PrintValues
  (bind _collectablesintrolevel (Variables|IntroLevel|GetCollectablesIntroLevel))
  ;[0.2344 0.2344 0.2344] Debug only, print save values
  (Development|PrintString 0 (Utilities|String|Append "Player Name: " (Utilities|String|ToString(Text) (Variables|Default|GetPlayerName))) true true "(R=0.000000,G=1.000000,B=0.053658,A=1.000000)" 1e+01)
  (Development|PrintString 0 (Utilities|String|Append "HighScore Intro Level: " (Utilities|String|ToString(Integer) (Variables|IntroLevel|GetHighScoreIntIntroLevel))) true true "(R=1.000000,G=0.153517,B=0.000000,A=1.000000)" 1e+01)
  (Development|PrintString 0 (Utilities|String|Append "Collectables on Intro Level: " (Utilities|String|ToString(Boolean) (Utilities|Array|Get(acopy) _collectablesintrolevel)) " " (Utilities|String|ToString(Boolean) (Utilities|Array|Get(acopy) _collectablesintrolevel 1)) " " (Utilities|String|ToString(Boolean) (Utilities|Array|Get(acopy) _collectablesintrolevel 2))) true true "(R=1.000000,G=0.903204,B=0.000000,A=1.000000)" 1e+01)
  (Development|PrintString 0 (Utilities|String|Append "High Score Intro Level: " (Utilities|String|ToString(Text) (Utilities|InttoText (Variables|IntroLevel|GetTutorialLevelScore)))) true true "(R=0.000000,G=0.774009,B=1.000000,A=1.000000)" 1e+01)
  (Development|PrintString 0 (Utilities|String|Append "Tutorial Level Rating: " (Utilities|String|ToString(Integer) (Variables|IntroLevel|GetIntroLevelRating))) true true "(R=0.417409,G=1.000000,B=0.000000,A=1.000000)" 1e+01)
  (Development|PrintString 0 (Utilities|String|Append "Level1 Rating: " (Utilities|String|ToString(Integer) (Variables|Level1|GetLevel1Rating))) true true "(R=1.000000,G=0.982960,B=0.363986,A=1.000000)" 1e+01)
  (bind _output_get (Variables|Default|SetDate (Math|DateTime|Now)))
  (Development|PrintString 0 (Utilities|String|Append (Utilities|String|ToString(Integer) (.day _output_get)) "." (Utilities|String|ToString(Integer) (.month _output_get)) "." (Utilities|String|ToString(Integer) (.year _output_get))) true true "(R=1.000000,G=0.396462,B=0.610220,A=1.000000)" 1e+01)
  (Development|PrintString 0 (Utilities|String|Append "Total highscore entries level 0: " (Utilities|String|ToString(Integer) (Variables|IntroLevel|GetHighScoreEntriesLevel0))) true true "(R=0.466406,G=1.000000,B=0.543420,A=1.000000)" 1e+01)
  (Development|PrintString 0 (Utilities|String|Append "Total highscore entries level 0: " (Utilities|String|ToString(Integer) (Utilities|Array|LastIndex (Variables|IntroLevel|GetPlayerScoresLevel0)))) true true "(R=0.402970,G=0.531121,B=1.000000,A=1.000000)" 1e+01)
  (for _array_element (Variables|IntroLevel|GetPlayerScoresLevel0)
    (for _array_element_2 (.Time (Utilities|Struct|BreakPlayerScoreLevel0 _array_element))
      (Development|PrintString 0 _array_element_2 true true "(R=0.349146,G=1.000000,B=0.568206,A=1.000000)")
      (for _array_element_3 (.Name (Utilities|Struct|BreakPlayerScoreLevel0 _array_element))
        (Development|PrintString 0 _array_element_3 true true "(R=0.349146,G=1.000000,B=0.568206,A=1.000000)"))
      (Development|PrintString 0 (Utilities|String|Append "Total highscore entries level 1: " (Utilities|String|ToString(Integer) (Utilities|Array|LastIndex (Variables|Level1|GetPlayerScoresLevel1)))) true true "(R=1.000000,G=0.263430,B=0.363237,A=1.000000)" 1e+01))))
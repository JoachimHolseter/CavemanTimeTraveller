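; Destructible wall that the Caveman smashes through while using his special, in both runner and puzzle modes.
; An overlap on TriggerBox checks the special, then once disables BlockVolume collision and shatters the Destructible with physics, radial damage and a delayed push.
; In the RunnerTest level, a Caveman or Cavewoman hitting the unbroken BlockVolume is marked dead.
; Characters are identified by object-name substring, and the level name selects the cast class.
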(event OnComponentBeginOverlap(TriggerBox)
  (params (OverlappedComponent :type Primitive%20Component%20Object%20Reference) (OtherActor :type Actor%20Object%20Reference) (OtherComp :type Primitive%20Component%20Object%20Reference) (OtherBodyIndex :type Integer) (bFromSweep :type Boolean) (SweepResult :type Hit%20Result%20Structure%20%28by%20ref%29))
  (if (Utilities|String|Contains (Utilities|GetObjectName OtherActor) "Caveman")
    (bind _returnvalue (Game|GetCurrentLevelName true))
    (if (Utilities|Enum|Equal(Enum) _returnvalue "RunnerTest")
      (bind _ascaveman_character_runner (Utilities|Casting|CastToCavemanCharacter_Runner OtherActor))
      (if (Variables|/Game/BP/CavemanCharacter_Runner.CavemanCharacter_Runner_C|GetUsingSpecial _ascaveman_character_runner)
        (Variables|Default|SetBoxBroken true :!label _label)
        (Utilities|FlowControl|DoOnce false
          (:Completed
            (Collision|SetCollisionProfileName (Variables|Default|GetBlockVolume) "NoCollision" :!class /Script/Engine.PrimitiveComponent)
            (Physics|SetSimulatePhysics (Variables|Default|GetDestructible) true)
            (Class|DestructibleComponent|ApplyRadiusDamage (Variables|Default|GetDestructible) 5.0 (Transformation|GetActorLocation) 0.0 5e+04 true)
            (Utilities|FlowControl|Delay 0.2)
            (Physics|AddForce (Variables|Default|GetDestructible) "1000.000000, 0, 0" "None" false))))
      (else
        (bind _ascaveman_character_puzzle (Utilities|Casting|CastToCavemanCharacter_Puzzle OtherActor))
        (if (Variables|/Game/BP/CavemanCharacter_Puzzle.CavemanCharacter_Puzzle_C|GetusingSpecial _ascaveman_character_puzzle)
          (goto _label))))))

(event OnComponentHit(BlockVolume)
  (params (HitComponent :type Primitive%20Component%20Object%20Reference) (OtherActor :type Actor%20Object%20Reference) (OtherComp :type Primitive%20Component%20Object%20Reference) (NormalImpulse :type Vector :default "0, 0, 0") (Hit :type Hit%20Result%20Structure%20%28by%20ref%29))
  (if (not (Variables|Default|GetBoxBroken))
    (if (Utilities|String|Contains (Utilities|GetObjectName OtherActor) "Caveman")
      (bind _returnvalue (Game|GetCurrentLevelName true))
      (if (Utilities|Enum|Equal(Enum) _returnvalue "RunnerTest")
        (bind _ascaveman_character_runner (Utilities|Casting|CastToCavemanCharacter_Runner OtherActor))
        (Variables|/Game/BP/CavemanCharacter_Runner.CavemanCharacter_Runner_C|SetisDead _ascaveman_character_runner true))
      (elif (Utilities|String|Contains (Utilities|GetObjectName OtherActor) "Cavewoman")
        (bind _returnvalue_2 (Game|GetCurrentLevelName true))
        (if (Utilities|Enum|Equal(Enum) _returnvalue_2 "RunnerTest")
          (bind _ascavewoman_character_runner (Utilities|Casting|CastToCavewomanCharacter_Runner OtherActor))
          (Variables|/Game/BP/CavewomanCharacter_Runner.CavewomanCharacter_Runner_C|SetisDead _ascavewoman_character_runner true))))))

(event EventBeginPlay)

(fn ConstructionScript)
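; BP_JungleStump is a jungle stump obstacle that kills the caveman or cavewoman runner character on impact in the RunnerTest level.
; Its capsule hit event passes through a DoOnce that is never reset, so only the first hit from any actor is evaluated.
; It identifies the character by object-name substring, checks the level name, then casts to the matching runner class and sets IsDead.
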(event OnComponentHit(Capsule)
  (params (HitComponent :type Primitive%20Component%20Object%20Reference) (OtherActor :type Actor%20Object%20Reference) (OtherComp :type Primitive%20Component%20Object%20Reference) (NormalImpulse :type Vector :default "0, 0, 0") (Hit :type Hit%20Result%20Structure%20%28by%20ref%29))
  (Utilities|FlowControl|DoOnce false
    (:Completed
      (if (Utilities|String|Contains (Utilities|GetObjectName OtherActor) "Caveman")
        (bind _returnvalue (Game|GetCurrentLevelName true))
        (if (Utilities|Enum|Equal(Enum) _returnvalue "RunnerTest")
          (bind _ascaveman_character_runner (Utilities|Casting|CastToCavemanCharacter_Runner OtherActor))
          (Variables|/Game/BP/CavemanCharacter/CavemanCharacter_Runner.CavemanCharacter_Runner_C|SetisDead _ascaveman_character_runner true))
        (elif (Utilities|String|Contains (Utilities|GetObjectName OtherActor) "Cavewoman")
          (bind _returnvalue_2 (Game|GetCurrentLevelName true))
          (if (Utilities|Enum|Equal(Enum) _returnvalue_2 "RunnerTest")
            (bind _ascavewoman_character_runner (Utilities|Casting|CastToCavewomanCharacter_Runner OtherActor))
            (Variables|/Game/BP/CavemanCharacter/CavewomanCharacter_Runner.CavewomanCharacter_Runner_C|SetisDead _ascavewoman_character_runner true)))))))

(fn ConstructionScript)